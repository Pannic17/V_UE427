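; BP_ky_fireTrail is a self-destroying fire trail effect that animates three trail components under a Scene component.
; On BeginPlay, a timeline spins Scene and, on each update, checks height and trail offset against thresholds.
; Two further timelines drive Scene's Z offset and the trails' X offset.
; Once Trail1's X reaches its threshold, the trails' relative location is set and the actor is destroyed after a short delay.
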(event `self.ReceiveBeginPlay`
  (bind _trail2 (`self.trail2`))
  (bind (_relativelocation_x _relativelocation_y _relativelocation_z) (`KismetMathLibrary.BreakVector` (`SceneComponent.RelativeLocation` (`self.Scene`))))
  (bind _relativelocation_x_2 (`KismetMathLibrary.BreakVector` (`SceneComponent.RelativeLocation` (`self.trail1`))))
  ;[1 1 1] move control
  (bind (_direction _rotation) (`Timeline|Timeline_0`)
    (:`Update`
      (`SceneComponent.K2_AddLocalRotation` (`self.Scene`) (`KismetMathLibrary.MakeRotator` 0.0 0.0 (* _rotation (stale `self.ReceiveTick` DeltaSeconds))) false false)
      (if (> _relativelocation_z 50.0)
        ;[1 1 1] z axis move control
        (bind (_direction_2 _float) (`Timeline|Timeline_2`)
          (:`Update`
            (`SceneComponent.K2_AddLocalOffset` (`self.Scene`) (`KismetMathLibrary.MakeVector` 0.0 0.0 (* _float (`GameplayStatics.GetWorldDeltaSeconds`))) false false)))
        (else
          ;[1 1 1] move stop
          (`SceneComponent.K2_SetRelativeLocation` (`self.Scene`) (0.0 0.0 0.0) false false)))
      ;[1 1 1] x axis move control
      (if (> _relativelocation_x_2 50.0)
        (bind (_direction_3 _location) (`Timeline|Timeline_1`)
          (:`Update`
            (`SceneComponent.K2_AddLocalOffset` _trail2 (`KismetMathLibrary.MakeVector` (* _location (`GameplayStatics.GetWorldDeltaSeconds`))) false false)
            (`SceneComponent.K2_AddLocalOffset` (`self.trail3`) (`KismetMathLibrary.MakeVector` (* _location (`GameplayStatics.GetWorldDeltaSeconds`))) false false)
            (`SceneComponent.K2_AddLocalOffset` (`self.trail1`) (`KismetMathLibrary.MakeVector` (* _location (`GameplayStatics.GetWorldDeltaSeconds`))) false false)))
        (else
          ;[1 1 1] move stop
          (`SceneComponent.K2_SetRelativeLocation` _trail2 (0.0 0.0 50.0) false false)
          (`SceneComponent.K2_SetRelativeLocation` (`self.trail3`) (0.0 0.0 50.0) false false)
          (`SceneComponent.K2_SetRelativeLocation` (`self.trail1`) (0.0 0.0 50.0) false false)
          ;[1 1 1] end
          (`KismetSystemLibrary.Delay` 1.0)
          (`self.K2_DestroyActor`))))))

(event `self.ReceiveTick`
  (params (DeltaSeconds :type "Float (single-precision)"))
  ;[1 1 1] move control
)

(fn `UserConstructionScript`)