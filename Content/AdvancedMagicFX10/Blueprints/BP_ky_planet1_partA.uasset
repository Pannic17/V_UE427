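; BP_ky_planet1_partA is the falling first stage of a planet magic effect from AdvancedMagicFX10.
; On BeginPlay, the MoveFX timeline drives frame-time-scaled local X and Z offsets on the Scene component.
; Once the Scene's relative Z drops to -30 or below, it spawns BP_ky_planet1_partB as the collision effect at the actor's transform and destroys itself, using a height threshold instead of collision detection.
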(event `self.ReceiveBeginPlay`
  (bind (_relativelocation_x _relativelocation_y _relativelocation_z) (`KismetMathLibrary.BreakVector` (`SceneComponent.RelativeLocation` (`self.Scene`))))
  ;[1 1 1] move control
  (bind (_direction _floatx _floatz) (`Timeline|moveFX`)
    (:`Update`
      (`SceneComponent.K2_AddLocalOffset` (`self.Scene`) (`KismetMathLibrary.MakeVector` (* _floatx (stale `self.ReceiveTick` DeltaSeconds)) 0.0 (* (stale `self.ReceiveTick` DeltaSeconds) _floatz)) false false)
      ;[1 1 1] spawn collision effect
      (if (not (> _relativelocation_z -30.0))
        (`|SpawnActorFromClass` "/Game/AdvancedMagicFX10/Blueprints/BP_ky_planet1_partB.BP_ky_planet1_partB_C" (`self.GetTransform` self) "Undefined" "OverrideRootScale" null null)
        ;[1 1 1] end
        (`self.K2_DestroyActor`)))))

(event `self.ReceiveTick`
  (params (DeltaSeconds :type "Float (single-precision)"))
  ;[1 1 1] move control
)

(fn `UserConstructionScript`)